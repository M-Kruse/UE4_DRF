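; BP_API_Door is a demo door actor that stays closed until a local web API reports it is online.
; On authority, a looping timer sends a GET heartbeat request, and its callback crudely string-parses the response into IsAPIOnline.
; Each tick checks that flag, which lags the asynchronous response, and prints a warning while false.
; Once true, a DoOnce plays a timeline that moves the mesh, then clears the timer on finish.
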(event Custom|SERVER_API_TestHeartbeat_EXAMPLE
  (Class|VaRestLibrary|CallURL (Utilities|String|Append "http://127.0.0.1:8000/api/heartbeat/" "") "GET" "x_www_form_urlencoded_body" 0 (delegate Custom|Callback_GetItemDetail)))

(event Custom|TIMELINE_OpenDoor
  (CallFunction|SERVERAPITestHeartbeatEXAMPLE)
  (if (Variables|Default|GetisAPIOnline)
    (CallFunction|SERVEROpenDemoDoor)
    (else
      (Development|PrintString "Door will remain closed until the API is online and GET requests are working"))))

(event Custom|Callback_GetItemDetail
  (params (Request :type Va%20Rest%20Request%20JSON%20Object%20Reference))
  (bind _returnvalue (Class|VaRestRequestJSON|GetResponseContentasString Request false))
  (Variables|Default|SetisAPIOnline (Utilities|Enum|Equal(Enum) (.RightS (Utilities|String|Split (Utilities|String|Replace (Utilities|String|Replace (Utilities|String|Replace (Utilities|String|Replace _returnvalue "[") "]") "{") "}") ":")) "true")))

(event Custom|SERVER_OpenDemoDoor
  (Utilities|FlowControl|DoOnce false
    (:Completed
      (bind _newtrack_0 (Timeline|Timeline_0 PlayFromStart)
        (:Update
          (Transformation|SetRelativeLocation (Variables|Default|GetStaticMesh) _newtrack_0 false false))
        (:Finished
          (Utilities|Time|ClearandInvalidateTimerbyHandle (Variables|Default|GetDoorMovementTimerHandle)))))))

(event EventBeginPlay
  (Networking|SwitchHasAuthority
    (:Authority
      (bind _returnvalue (Utilities|Time|SetTimerbyEvent (delegate Custom|TIMELINE_OpenDoor) 1.0 true))
      (Variables|Default|SetDoorMovementTimerHandle _returnvalue))))

(fn ConstructionScript)